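; Actor that lets the player click UI widgets through a Widget Interaction component, in a custom map's widget menu.
; Holding ScoreboardLeft unhides the root component and its children and sets an Open flag; releasing it hides them and clears the flag.
; TriggerRight acts as the left mouse button on the interaction component, pressing only while Open but always releasing.
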(event `InputAction|ScoreboardLeft` :consume false
  (params (Key :type "Key Structure"))
  (:`Pressed`
    (`SceneComponent.SetHiddenInGame` (`self.DefaultSceneRoot`) false true)
    (set `self.Open?` true))
  (:`Released`
    (`SceneComponent.SetHiddenInGame` (`self.DefaultSceneRoot`) true true)
    (set `self.Open?` false)))

(event `InputAction|TriggerRight` :consume false
  (params (Key :type "Key Structure"))
  (:`Pressed`
    (if (`self.Open?`)
      (`WidgetInteractionComponent.PressPointerKey` (`self.WidgetInteraction`) "LeftMouseButton")))
  (:`Released`
    (`WidgetInteractionComponent.ReleasePointerKey` (`self.WidgetInteraction`) "LeftMouseButton")))

(fn `UserConstructionScript`)