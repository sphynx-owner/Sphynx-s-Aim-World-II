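; Base target for an aim-training practice, supporting hit and tracking modes, each with an optional health variant.
; Tick drives lifespan, health drain and clamped movement through a child-actor movement controller, and reports time-on-target to MainBlueprint.
; Head hits and laser overlaps count only while PlayerMoving is true; overlaps recolor tracked targets.
; Outcomes pass parameter structs to RunSequnce for scoring, sequence advance or destruction, with empty SelSeq stubs for self-sequencing.
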(event `self.ReceiveBeginPlay`
  (`SceneComponent.SetVisibility` (`self.Body`) (`self.HasBody?`) false)
  (set `self.SpawnLocation` (`SceneComponent.K2_GetComponentLocation` (`self.DefaultSceneRoot`)))
  (if (`self.IsBlueOnTrack?`)
    (set `self.TrackBaseMaterial` "/Game/CustomMaps/UGC2842012712/Materials/M_Blue.M_Blue")
    (else
      (set `self.TrackBaseMaterial` "/Game/CustomMaps/UGC2842012712/Materials/M_Red.M_Red")))
  (`self.SetIsTrack`)
  (bind _astarget_movement_controller (cast `/Game/CustomMaps/UGC2842012712/Blueprints/Practices/TargetMovementController` (`ChildActorComponent.ChildActor` (`self.TargetMovementController`))))
  (set `self.MovementController` _astarget_movement_controller)
  (if (`self.SelfSeqInitiateOnSpawn?`)
    (`self.SelSeqInitiate`)))

(event `self.ReceiveTick`
  (params (DeltaSeconds :type "Float (single-precision)"))
  (bind _mainblueprint (`self.MainBlueprint`))
  (`self.CheckPlayerMoving`)
  (if (`/Game/CustomMaps/UGC2842012712/Blueprints/Practices/PracticeTemplate.PracticeRunning?` (`self.MainBlueprint`))
    (`self.LifeSpanning` DeltaSeconds)
    (`self.TrackTarget` DeltaSeconds)
    (`self.Move` DeltaSeconds)
    (switch `/Game/CustomMaps/UGC2842012712/Blueprints/Global/Enums/TargetState` (`self.TargetState`)
      (:`NewEnumerator3`
        _)
      (:`NewEnumerator4`
        _))
    (if (`/Game/CustomMaps/UGC2842012712/Blueprints/Practices/PracticeTemplate.MeasureTOT?` _mainblueprint)
      (`KismetSystemLibrary.Delay` 0.07)
      (`/Game/CustomMaps/UGC2842012712/Blueprints/Practices/PracticeTemplate.Track` (`self.MainBlueprint`) (`self.PlaySoundOnTarget`) (`self.IsColliding?`) (`self.PlaySoundOffTarget`) self)
      (else
        (set `/Game/CustomMaps/UGC2842012712/Blueprints/Practices/PracticeTemplate.MeasureTOT?` true _mainblueprint)))))

(event `self.Head.OnComponentHit`
  (params (HitComponent :type "PrimitiveComponent Object Reference") (OtherActor :type "Actor Object Reference") (OtherComp :type "PrimitiveComponent Object Reference") (NormalImpulse :type "Vector Structure") (Hit :type "HitResult Structure (by ref)"))
  (if (`/Game/CustomMaps/UGC2842012712/Blueprints/Practices/PracticeTemplate.PracticeRunning?` (`self.MainBlueprint`))
    (if (not (`/Game/CustomMaps/UGC2842012712/Blueprints/Practices/PracticeTemplate.IsHitScan?` (`self.MainBlueprint`)))
      (`self.TargetHit`))))

(event `self.Head.OnComponentBeginOverlap`
  (params (OverlappedComponent :type "PrimitiveComponent Object Reference") (OtherActor :type "Actor Object Reference") (OtherComp :type "PrimitiveComponent Object Reference") (OtherBodyIndex :type Integer) (bFromSweep :type Boolean) (SweepResult :type "HitResult Structure (by ref)"))
  (cast `/Game/CustomMaps/UGC2842012712/Blueprints/lazer` OtherActor)
  (`self.StartColliding`))

(event `self.Head.OnComponentEndOverlap`
  (params (OverlappedComponent :type "PrimitiveComponent Object Reference") (OtherActor :type "Actor Object Reference") (OtherComp :type "PrimitiveComponent Object Reference") (OtherBodyIndex :type Integer))
  (cast `/Game/CustomMaps/UGC2842012712/Blueprints/lazer` OtherActor)
  (`self.StopColliding`))

(fn `CheckPlayerMoving`
  (bind _returnvalue (`SceneComponent.K2_GetComponentLocation` (`/Game/CustomMaps/UGC2842012712/Blueprints/Practices/PracticeTemplate.PlayerLocation` (`self.MainBlueprint`))))
  (if (`self.IsCheckingMovement?`)
    (if (== _returnvalue (`self.PlayerPreviousLocation`))
      (set `self.PlayerMoving?` false)
      (else
        (set `self.PlayerMoving?` true)
        (set `self.PlayerPreviousLocation` _returnvalue)))))

(fn `LifeSpanning`
  (params (DeltaTime :type "Float (double-precision)"))
  (if (`self.HasLifeSpan?`)
    (set `self.Life` (`KismetMathLibrary.FInterpTo_Constant` (`self.Life`) 0.0 DeltaTime 1.0))
    (if (== (`self.Life`) 0.0)
      (`/Engine/EditorBlueprintResources/StandardMacros.DoOnce` false :!label _label
        (:`Completed`
          (`self.RunSequnce` (`self.LateReact`))))
      (else
        (goto _label :!via `Reset`)))))

(fn `Move`
  (params (DeltaTime :type "Float (double-precision)"))
  (if (`self.IsMoving?`)
    (`/Game/CustomMaps/UGC2842012712/Blueprints/Practices/TargetMovementController.TickMovement` (`self.MovementController`) (`self.DefaultSceneRoot`) DeltaTime)
    (`SceneComponent.K2_SetWorldLocation` (`self.DefaultSceneRoot`) (`self.ClampLocation` (`SceneComponent.K2_GetComponentLocation` (`self.DefaultSceneRoot`))) false false)))

(fn `Randomise`
  (bind _returnvalue (`KismetMathLibrary.RandomFloatInRange` 0.0 1.0))
  (if (`self.HasBody?`)
    (`SceneComponent.SetWorldScale3D` (`self.DefaultSceneRoot`) (`KismetMathLibrary.Conv_DoubleToVector` 0.2))
    (else
      (`SceneComponent.SetWorldScale3D` (`self.DefaultSceneRoot`) (`KismetMathLibrary.Conv_DoubleToVector` (`KismetMathLibrary.RandomFloatInRange` 0.2 0.6)))))
  (set `self.IsMoving?` (> _returnvalue 0.5))
  (if (> _returnvalue 0.5)
    (set `self.TargetState` "NewEnumerator3"))
  (`self.SetIsTrack`))

(fn `RandomiseMovementAngle`
  (bind _returnvalue (`KismetMathLibrary.RandomFloatInRange` -20.0 20.0))
  (bind _movementcontroller (`self.MovementController`))
  (if (`KismetMathLibrary.RandomBool`)
    (set `/Game/CustomMaps/UGC2842012712/Blueprints/Practices/TargetMovementController.Rotation` (`KismetMathLibrary.MakeRotator` 0.0 _returnvalue 180.0) _movementcontroller)
    (else
      (set `/Game/CustomMaps/UGC2842012712/Blueprints/Practices/TargetMovementController.Rotation` (`KismetMathLibrary.MakeRotator` 0.0 _returnvalue) _movementcontroller))))

(fn `ResetVariables`
  (params (HealthScale :type "Float (double-precision)" :default 1.0) (Life :type "Float (double-precision)" :default 1.0) (Health :type Integer :default 0))
  (bind _scene (`self.Scene`))
  (bind (_relativescale3d_x _relativescale3d_y _relativescale3d_z) (`KismetMathLibrary.BreakVector` (`SceneComponent.RelativeScale3D` _scene)))
  (set `self.Health Scale` HealthScale)
  (`SceneComponent.SetRelativeScale3D` _scene (`KismetMathLibrary.MakeVector` _relativescale3d_x (`self.Health Scale`) _relativescale3d_z))
  (set `self.Life` Life)
  (set `self.Health` Health)
  (switch `/Game/CustomMaps/UGC2842012712/Blueprints/Global/Enums/TargetState` (`self.TargetState`)
    (:`NewEnumerator4`
      (`SceneComponent.SetVisibility` (`self.HealthBar`) (`self.ShowTrackHealth?`) false))))

(fn `RunSequnce`
  (params (TargetParameter :type "/Game/CustomMaps/UGC2842012712/Blueprints/Global/Structs/TargetPrarameter Structure") (`Hit?` :type Boolean))
  (bind (_true_ _hit_ _playsound_ _selseq_ _seq_ _destroy_) (break `/Game/CustomMaps/UGC2842012712/Blueprints/Global/Structs/TargetPrarameter` TargetParameter))
  (if _hit_
    (`/Game/CustomMaps/UGC2842012712/Blueprints/Practices/PracticeTemplate.Hit` (`self.MainBlueprint`) `Hit?` 600.0 _playsound_ self))
  (if _selseq_
    (`self.SelSeqInitiate`))
  (if _seq_
    (`/Game/CustomMaps/UGC2842012712/Blueprints/Practices/PracticeTemplate.Initiatepractice` (`self.MainBlueprint`) self))
  (if _destroy_
    (`self.K2_DestroyActor`)))

(fn `SelSeq1`)

(fn `SelSeq2`)

(fn `SelSeq3`)

(fn `SelSeqInitiate`
  (set `self.SelSeqNumber` (mod (`self.SelSeqNumber`) (`self.SelSeqLength`)))
  (`/Engine/EditorBlueprintResources/StandardMacros.IncrementInt` (`self.SelSeqNumber`)
    (:`  `
      (if (== (`self.SelSeqNumber`) 1)
        (`self.SelSeq1`)
        (elif (== (`self.SelSeqNumber`) 2)
          (`self.SelSeq2`)
          (elif (== (`self.SelSeqNumber`) 3)
            (`self.SelSeq3`)))))))

(fn `SetIsTrack`
  (bind _body (`self.Body`))
  (bind _trackbasematerial (`self.TrackBaseMaterial`))
  (bind _body_2 (`self.Body`))
  (switch `/Game/CustomMaps/UGC2842012712/Blueprints/Global/Enums/TargetState` (`self.TargetState`)
    (:`NewEnumerator0`
      (`PrimitiveComponent.SetMaterial` (`self.Head`) 0 "/Game/CustomMaps/UGC2842012712/Materials/M_Red.M_Red" :!label _label)
      (`PrimitiveComponent.SetMaterial` _body_2 0 "/Game/CustomMaps/UGC2842012712/Materials/M_Red.M_Red")
      (`PrimitiveComponent.SetMaterial` _body_2 1 "/Game/CustomMaps/UGC2842012712/Materials/M_Red.M_Red")
      (`PrimitiveComponent.SetMaterial` _body_2 2 "/Game/CustomMaps/UGC2842012712/Materials/M_Red.M_Red")
      (`SceneComponent.SetVisibility` (`self.HealthBar`) false false)
      (set `/Game/CustomMaps/UGC2842012712/Blueprints/Practices/PracticeTemplate.MeasureTOT?` false (`self.MainBlueprint`)))
    (:`NewEnumerator1`
      (goto _label))
    (:`NewEnumerator2`
      (goto _label))
    (:`NewEnumerator3`
      (`PrimitiveComponent.SetMaterial` (`self.Head`) 0 _trackbasematerial :!label _label_2)
      (`PrimitiveComponent.SetMaterial` _body 0 _trackbasematerial)
      (`PrimitiveComponent.SetMaterial` _body 1 _trackbasematerial)
      (`PrimitiveComponent.SetMaterial` _body 2 _trackbasematerial)
      (switch `/Game/CustomMaps/UGC2842012712/Blueprints/Global/Enums/TargetState` (`self.TargetState`)
        (:`NewEnumerator4`
          (if (`self.ShowTrackHealth?`)
            (`SceneComponent.SetVisibility` (`self.HealthBar`) true false)))))
    (:`NewEnumerator4`
      (goto _label_2))))

(fn `StartColliding`
  (bind _body (`self.Body`))
  (if (`self.PlayerMoving?`)
    (set `self.IsColliding?` true)
    (switch `/Game/CustomMaps/UGC2842012712/Blueprints/Global/Enums/TargetState` (`self.TargetState`)
      (:`NewEnumerator3`
        _)
      (:`NewEnumerator4`
        _))
    (set `/Game/CustomMaps/UGC2842012712/Blueprints/Practices/PracticeTemplate.IsColliding?` true (`self.MainBlueprint`))
    (`PrimitiveComponent.SetMaterial` (`self.Head`) 0 "/Game/CustomMaps/UGC2842012712/Materials/M_Green.M_Green")
    (`PrimitiveComponent.SetMaterial` _body 0 "/Game/CustomMaps/UGC2842012712/Materials/M_Green.M_Green")
    (`PrimitiveComponent.SetMaterial` _body 1 "/Game/CustomMaps/UGC2842012712/Materials/M_Green.M_Green")
    (`PrimitiveComponent.SetMaterial` _body 2 "/Game/CustomMaps/UGC2842012712/Materials/M_Green.M_Green")
    (switch `/Game/CustomMaps/UGC2842012712/Blueprints/Global/Enums/TargetState` (`self.TargetState`)
      (:`NewEnumerator4`
        (`SceneComponent.SetVisibility` (`self.HealthBar`) true false)))))

(fn `StopColliding`
  (bind _body (`self.Body`))
  (bind _trackbasematerial (`self.TrackBaseMaterial`))
  (if (`self.PlayerMoving?`)
    (set `self.IsColliding?` false)
    (switch `/Game/CustomMaps/UGC2842012712/Blueprints/Global/Enums/TargetState` (`self.TargetState`)
      (:`NewEnumerator3`
        _)
      (:`NewEnumerator4`
        _))
    (set `/Game/CustomMaps/UGC2842012712/Blueprints/Practices/PracticeTemplate.IsColliding?` false (`self.MainBlueprint`))
    (`PrimitiveComponent.SetMaterial` (`self.Head`) 0 _trackbasematerial)
    (`PrimitiveComponent.SetMaterial` _body 0 _trackbasematerial)
    (`PrimitiveComponent.SetMaterial` _body 1 _trackbasematerial)
    (`PrimitiveComponent.SetMaterial` _body 2 _trackbasematerial)))

(fn `TargetHit`
  (bind _health (`self.Health`))
  (if (`self.PlayerMoving?`)
    (switch `/Game/CustomMaps/UGC2842012712/Blueprints/Global/Enums/TargetState` (`self.TargetState`)
      (:`NewEnumerator1`
        (`self.RunSequnce` (`self.React`) true :!label _label))
      (:`NewEnumerator2`
        (`/Engine/EditorBlueprintResources/StandardMacros.DecrementInt` _health
          (:`  `
            (if (> _health 0)
              (`self.RunSequnce` (`self.HealthReact`) true)
              (else
                (goto _label)))))))))

(fn `TrackTarget`
  (params (DeltaTime :type "Float (double-precision)"))
  (bind _scene (`self.Scene`))
  (bind (_relativescale3d_x _relativescale3d_y _relativescale3d_z) (`KismetMathLibrary.BreakVector` (`SceneComponent.RelativeScale3D` _scene)))
  (switch `/Game/CustomMaps/UGC2842012712/Blueprints/Global/Enums/TargetState` (`self.TargetState`)
    (:`NewEnumerator4`
      (if (and (`self.IsColliding?`) (`self.PlayerMoving?`))
        (set `self.Health Scale` (`KismetMathLibrary.FInterpTo_Constant` (`self.Health Scale`) 0.0 DeltaTime (`self.HealthSpeed`)))
        (`SceneComponent.SetRelativeScale3D` _scene (`KismetMathLibrary.MakeVector` _relativescale3d_x (`self.Health Scale`) _relativescale3d_z))
        (if (== (`self.Health Scale`) 0.0)
          (`/Engine/EditorBlueprintResources/StandardMacros.DoOnce` false :!label _label
            (:`Completed`
              (`self.RunSequnce` (`self.React`) true)))
          (else
            (goto _label :!via `Reset`)))))))

(fn `UserConstructionScript`
  (`SceneComponent.SetVisibility` (`self.Body`) (`self.HasBody?`) false))