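; Reusable target mover that drives a passed-in root component by one of several movement states, apparently for practice maps.
; TickMovement selects angular, inertial, gravitation, spherical or cylindrical orbit, or eased location or rotation interpolation.
; Most modes build MovementVector, apply it to world location and mirror it on Sphere1; location interpolation sets position directly.
; DoOnce gates completion events, though rotation completion also fires ReachedLocation, leaving ReachedRotation unused.
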(event `ReachedLocation`)

(event `ReachedRotation`)

(fn `TickMovement`
  (params (RootComponent :type "SceneComponent Object Reference") (DeltaTime :type "Float (double-precision)"))
  (switch `/Game/CustomMaps/UGC2842012712/Blueprints/Global/Enums/MovementState` (`self.MovementState`)
    (:`NewEnumerator0`
      (`self.MoveAngular`
        (:`out`
          (`SceneComponent.K2_SetWorldLocation` RootComponent (+ (* (`self.MovementVector`) (* DeltaTime 100.0)) (`SceneComponent.K2_GetComponentLocation` RootComponent)) false false :!label _label)
          (`SceneComponent.K2_SetRelativeLocation` (`self.Sphere1`) (`self.MovementVector`) false false :!label _label_2))))
    (:`NewEnumerator1`
      (`self.MoveAngularInn` DeltaTime
        (:`out`
          (goto _label))))
    (:`NewEnumerator2`
      (`self.Gravitate` DeltaTime
        (:`Out`
          (goto _label))))
    (:`NewEnumerator3`
      (`self.Radial` true RootComponent DeltaTime
        (:`out`
          (`SceneComponent.K2_SetWorldLocation` RootComponent (+ (`self.MovementVector`) (`SceneComponent.K2_GetComponentLocation` RootComponent)) false false :!label _label_3)
          (goto _label_2))))
    (:`NewEnumerator6`
      (`self.Radial` false RootComponent DeltaTime
        (:`out`
          (goto _label_3))))
    (:`NewEnumerator4`
      (`self.TowardsLocationInterp` RootComponent DeltaTime
        (:`Done`
          (`/Engine/EditorBlueprintResources/StandardMacros.DoOnce` false :!label _label_4
            (:`Completed`
              (`self.ReachedLocation`))))
        (:`YetToReach`
          (goto _label_4 :!via `Reset`))))
    (:`NewEnumerator5`
      (`self.TowardsRotationInterp` DeltaTime
        (:`Done`
          (`/Engine/EditorBlueprintResources/StandardMacros.DoOnce` false :!label _label_5
            (:`Completed`
              (`self.ReachedLocation`))))
        (:`YetToReach`
          (`|ExecutionSequence`
            (:`then_0`
              (goto _label_5 :!via `Reset`))
            (:`then_1`
              (`self.MoveAngular`
                (:`out`
                  (goto _label))))))))))

(fn `UserConstructionScript`)