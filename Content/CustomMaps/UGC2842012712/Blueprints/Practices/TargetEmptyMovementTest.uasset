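; Test variant of an aim-practice target whose movement is driven by a child-actor TargetMovementController.
; BeginPlay gives the controller a movement state and one fixed gravitator point, and Tick only advances that movement on the scene root while IsMoving.
; Functions for hit, tracking health, lifespan and randomisation exist but are not called here; their reactions route through RunSequnce to sequences or destruction.
; SelSeq steps are empty stubs, and collision highlight materials are disconnected.
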(event `self.ReceiveBeginPlay`
  (bind _astarget_movement_controller (cast `/Game/CustomMaps/UGC2842012712/Blueprints/Practices/TargetMovementController` (`ChildActorComponent.ChildActor` (`self.TargetMovementController`))))
  (bind _output_get (set `self.MovementController` _astarget_movement_controller))
  (set `/Game/CustomMaps/UGC2842012712/Blueprints/Practices/TargetMovementController.MovementState` "NewEnumerator2" _output_get)
  (set `/Game/CustomMaps/UGC2842012712/Blueprints/Practices/TargetMovementController.Gravitators` (`|MakeArray` (-450.0 -8420.0 530.0) :!type "Vector Structure") _output_get))

(event `self.ReceiveTick`
  (params (DeltaSeconds :type "Float (single-precision)"))
  (`self.Move` DeltaSeconds))

(fn `CheckPlayerMoving`)

(fn `LifeSpanning`
  (params (DeltaTime :type "Float (double-precision)"))
  (if (`self.HasLifeSpan?`)
    (set `self.Life` (`KismetMathLibrary.FInterpTo_Constant` (`self.Life`) 0.0 DeltaTime 1.0))
    (if (== (`self.Life`) 0.0)
      (`/Engine/EditorBlueprintResources/StandardMacros.DoOnce` false :!label _label
        (:`Completed`
          (`self.RunSequnce` (`self.LateReact`))))
      (else
        (goto _label :!via `Reset`)))))

(fn `Move`
  (params (DeltaTime :type "Float (double-precision)"))
  (if (`self.IsMoving?`)
    (`/Game/CustomMaps/UGC2842012712/Blueprints/Practices/TargetMovementController.TickMovement` (`self.MovementController`) (`self.DefaultSceneRoot`) DeltaTime)
    (`SceneComponent.K2_SetWorldLocation` (`self.DefaultSceneRoot`) (`SceneComponent.K2_GetComponentLocation` (`self.DefaultSceneRoot`)) false false)))

(fn `Randomise`
  (bind _returnvalue (`KismetMathLibrary.RandomFloatInRange` 0.0 1.0))
  (if (`self.HasBody?`)
    (`SceneComponent.SetWorldScale3D` (`self.DefaultSceneRoot`) (`KismetMathLibrary.Conv_DoubleToVector` 0.2))
    (else
      (`SceneComponent.SetWorldScale3D` (`self.DefaultSceneRoot`) (`KismetMathLibrary.Conv_DoubleToVector` (`KismetMathLibrary.RandomFloatInRange` 0.2 0.6)))))
  (set `self.IsMoving?` (> _returnvalue 0.5))
  (if (> _returnvalue 0.5)
    (set `self.TargetState` "NewEnumerator3"))
  (`self.SetIsTrack`))

(fn `RandomiseMovementAngle`
  (bind _returnvalue (`KismetMathLibrary.RandomFloatInRange` -20.0 20.0))
  (bind _movementcontroller (`self.MovementController`))
  (if (`KismetMathLibrary.RandomBool`)
    (set `/Game/CustomMaps/UGC2842012712/Blueprints/Practices/TargetMovementController.Rotation` (`KismetMathLibrary.MakeRotator` 0.0 _returnvalue 180.0) _movementcontroller)
    (else
      (set `/Game/CustomMaps/UGC2842012712/Blueprints/Practices/TargetMovementController.Rotation` (`KismetMathLibrary.MakeRotator` 0.0 _returnvalue) _movementcontroller))))

(fn `ResetVariables`
  (params (HealthScale :type "Float (double-precision)" :default 1.0) (Life :type "Float (double-precision)" :default 1.0) (Health :type Integer :default 0))
  (bind _scene (`self.Scene`))
  (bind (_relativescale3d_x _relativescale3d_y _relativescale3d_z) (`KismetMathLibrary.BreakVector` (`SceneComponent.RelativeScale3D` _scene)))
  (set `self.Health Scale` HealthScale)
  (`SceneComponent.SetRelativeScale3D` _scene (`KismetMathLibrary.MakeVector` _relativescale3d_x (`self.Health Scale`) _relativescale3d_z))
  (set `self.Life` Life)
  (set `self.Health` Health)
  (switch `/Game/CustomMaps/UGC2842012712/Blueprints/Global/Enums/TargetState` (`self.TargetState`)
    (:`NewEnumerator4`
      (`SceneComponent.SetVisibility` (`self.HealthBar`) (`self.ShowTrackHealth?`) false))))

(fn `RunSequnce`
  (params (TargetParameter :type "/Game/CustomMaps/UGC2842012712/Blueprints/Global/Structs/TargetPrarameter Structure") (`Hit?` :type Boolean))
  (bind (_true_ _hit_ _playsound_ _selseq_ _seq_ _destroy_) (break `/Game/CustomMaps/UGC2842012712/Blueprints/Global/Structs/TargetPrarameter` TargetParameter))
  (if (not _hit_)
    (if _selseq_
      (`self.SelSeqInitiate`))
    (if _seq_
      _
      (elif _destroy_
        (`self.K2_DestroyActor`)))))

(fn `SelSeq1`)

(fn `SelSeq2`)

(fn `SelSeq3`)

(fn `SelSeqInitiate`
  (set `self.SelSeqNumber` (mod (`self.SelSeqNumber`) (`self.SelSeqLength`)))
  (`/Engine/EditorBlueprintResources/StandardMacros.IncrementInt` (`self.SelSeqNumber`)
    (:`  `
      (if (== (`self.SelSeqNumber`) 1)
        (`self.SelSeq1`)
        (elif (== (`self.SelSeqNumber`) 2)
          (`self.SelSeq2`)
          (elif (== (`self.SelSeqNumber`) 3)
            (`self.SelSeq3`)))))))

(fn `SetIsTrack`
  (bind _body (`self.Body`))
  (bind _trackbasematerial (`self.TrackBaseMaterial`))
  (switch `/Game/CustomMaps/UGC2842012712/Blueprints/Global/Enums/TargetState` (`self.TargetState`)
    (:`NewEnumerator0`)
    (:`NewEnumerator1`)
    (:`NewEnumerator2`)
    (:`NewEnumerator3`
      _)
    (:`NewEnumerator4`
      _))
  (`PrimitiveComponent.SetMaterial` (`self.Head`) 0 _trackbasematerial)
  (`PrimitiveComponent.SetMaterial` _body 0 _trackbasematerial)
  (`PrimitiveComponent.SetMaterial` _body 1 _trackbasematerial)
  (`PrimitiveComponent.SetMaterial` _body 2 _trackbasematerial)
  (switch `/Game/CustomMaps/UGC2842012712/Blueprints/Global/Enums/TargetState` (`self.TargetState`)
    (:`NewEnumerator4`
      (if (`self.ShowTrackHealth?`)
        (`SceneComponent.SetVisibility` (`self.HealthBar`) true false)))))

(fn `StartColliding`
  (if (`self.PlayerMoving?`)
    (set `self.IsColliding?` true)
    (switch `/Game/CustomMaps/UGC2842012712/Blueprints/Global/Enums/TargetState` (`self.TargetState`))))

(fn `StopColliding`
  (if (`self.PlayerMoving?`)
    (set `self.IsColliding?` false)
    (switch `/Game/CustomMaps/UGC2842012712/Blueprints/Global/Enums/TargetState` (`self.TargetState`))))

(fn `TargetHit`
  (bind _health (`self.Health`))
  (if (`self.PlayerMoving?`)
    (switch `/Game/CustomMaps/UGC2842012712/Blueprints/Global/Enums/TargetState` (`self.TargetState`)
      (:`NewEnumerator1`
        (`self.RunSequnce` (`self.React`) true :!label _label))
      (:`NewEnumerator2`
        (`/Engine/EditorBlueprintResources/StandardMacros.DecrementInt` _health
          (:`  `
            (if (> _health 0)
              (`self.RunSequnce` (`self.HealthReact`) true)
              (else
                (goto _label)))))))))

(fn `TrackTarget`
  (params (DeltaTime :type "Float (double-precision)"))
  (bind _scene (`self.Scene`))
  (bind (_relativescale3d_x _relativescale3d_y _relativescale3d_z) (`KismetMathLibrary.BreakVector` (`SceneComponent.RelativeScale3D` _scene)))
  (switch `/Game/CustomMaps/UGC2842012712/Blueprints/Global/Enums/TargetState` (`self.TargetState`)
    (:`NewEnumerator4`
      (if (and (`self.IsColliding?`) (`self.PlayerMoving?`))
        (set `self.Health Scale` (`KismetMathLibrary.FInterpTo_Constant` (`self.Health Scale`) 0.0 DeltaTime (`self.HealthSpeed`)))
        (`SceneComponent.SetRelativeScale3D` _scene (`KismetMathLibrary.MakeVector` _relativescale3d_x (`self.Health Scale`) _relativescale3d_z))
        (if (== (`self.Health Scale`) 0.0)
          (`/Engine/EditorBlueprintResources/StandardMacros.DoOnce` false :!label _label
            (:`Completed`
              (`self.RunSequnce` (`self.React`) true)))
          (else
            (goto _label :!via `Reset`)))))))

(fn `UserConstructionScript`
  (`SceneComponent.SetVisibility` (`self.Body`) (`self.HasBody?`) false))