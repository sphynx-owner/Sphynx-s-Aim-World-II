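; Test child of a practice template Blueprint that runs a timed target-clearing exercise.
; BeginPlay sets its target class, and Sequence1 spawns a batch of targets at loose random offsets around the anchor, passing each an index and a back-reference.
; Sequence2 removes a given target from the list and calls StopwatchFinished once none remain.
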(event `self.ReceiveBeginPlay`
  (`parent.ReceiveBeginPlay`)
  (set `self.TargetClass` "/Game/CustomMaps/UGC2842012712/Blueprints/Practices/TargetTemplateTestChild.TargetTemplateTestChild_C"))

(event `self.Sequence1`
  (params (Target :type "/Game/CustomMaps/UGC2842012712/Blueprints/Practices/TargetTemplate Object Reference"))
  (for _index (range 21)
    (bind _location (`self.TDRandomLocationLoose` _index))
    (bind _returnvalue (`|SpawnActorFromClass` "/Game/CustomMaps/UGC2842012712/Blueprints/Practices/TargetTemplateTestChild.TargetTemplateTestChild_C" (`KismetMathLibrary.MakeTransform` (+ _location (`SceneComponent.K2_GetComponentLocation` (`self.Anchor`))) (struct) (`KismetMathLibrary.Conv_DoubleToVector` (`self.TargetSize`))) "Undefined" "OverrideRootScale" null false false false true false 1.0 1.0 1.0 5 true false false false 1 true _index self 3000.0 1200.0 1000.0 -3000.0 -1200.0 -1000.0 "NewEnumerator1" (make `/Game/CustomMaps/UGC2842012712/Blueprints/Global/Structs/TargetPrarameter` false true true true false true) (struct) (struct) null))
    (`KismetArrayLibrary.Array_Set` (`self.Targets`) _index _returnvalue true)))

(event `self.Sequence2`
  (params (Target :type "/Game/CustomMaps/UGC2842012712/Blueprints/Practices/TargetTemplate Object Reference"))
  (bind _targets (`self.Targets`))
  (`KismetArrayLibrary.Array_RemoveItem` _targets Target)
  (if (== (`KismetArrayLibrary.Array_Length` _targets) 0)
    (`self.StopwatchFinished`)))

(fn `UserConstructionScript`
  (`parent.UserConstructionScript`))