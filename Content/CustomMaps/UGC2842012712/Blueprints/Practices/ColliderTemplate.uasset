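; Target collider for a practice map, run as a child actor of a PracticeTemplate that must be held under a lazer actor.
; While the parent's TimeRunning is set, Tick counts a randomized hold time down only during lazer overlap, pausing otherwise.
; At zero it calls Initiatepractice on the parent and rerolls the time, with DoOnce nodes guarding both steps.
; The cube turns green during overlap as feedback.
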(event `self.ReceiveTick`
  (params (DeltaSeconds :type "Float (single-precision)"))
  (if (`/Game/CustomMaps/UGC2842012712/Blueprints/Practices/PracticeTemplate.TimeRunning?` (`self.MainBlueprint`))
    (`|ExecutionSequence`
      (:`then_0`
        (`/Engine/EditorBlueprintResources/StandardMacros.DoOnce` false :!label _label
          (:`Completed`
            (`self.ResetTime`))))
      (:`then_1`
        (if (`self.IsColliding?`)
          (set `self.Time` (`KismetMathLibrary.FInterpTo_Constant` (`self.Time`) 0.0 DeltaSeconds 1.0))
          (if (== (`self.Time`) 0.0)
            (`/Engine/EditorBlueprintResources/StandardMacros.DoOnce` false :!label _label_2
              (:`Completed`
                (`/Game/CustomMaps/UGC2842012712/Blueprints/Practices/PracticeTemplate.Initiatepractice` (`self.MainBlueprint`) null)
                (`self.ResetTime`)))))))
    (else
      (goto _label :!via `Reset`))))

(event `ResetTime`
  (set `self.Time` (`KismetMathLibrary.RandomFloatInRange` 1.0 4.0))
  (goto _label_2 :!via `Reset`))

(event `self.Cube.OnComponentBeginOverlap`
  (params (OverlappedComponent :type "PrimitiveComponent Object Reference") (OtherActor :type "Actor Object Reference") (OtherComp :type "PrimitiveComponent Object Reference") (OtherBodyIndex :type Integer) (bFromSweep :type Boolean) (SweepResult :type "HitResult Structure (by ref)"))
  (cast `/Game/CustomMaps/UGC2842012712/Blueprints/lazer` OtherActor)
  (set `self.IsColliding?` true)
  (`PrimitiveComponent.SetMaterial` (`self.Cube`) 0 "/Game/CustomMaps/UGC2842012712/Materials/M_Green.M_Green"))

(event `self.Cube.OnComponentEndOverlap`
  (params (OverlappedComponent :type "PrimitiveComponent Object Reference") (OtherActor :type "Actor Object Reference") (OtherComp :type "PrimitiveComponent Object Reference") (OtherBodyIndex :type Integer))
  (cast `/Game/CustomMaps/UGC2842012712/Blueprints/lazer` OtherActor)
  (set `self.IsColliding?` false)
  (`PrimitiveComponent.SetMaterial` (`self.Cube`) 0 null))

(fn `UserConstructionScript`
  (bind _aspractice_template (cast `/Game/CustomMaps/UGC2842012712/Blueprints/Practices/PracticeTemplate` (`self.GetParentActor`)))
  (set `self.MainBlueprint` _aspractice_template))