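; Pavlov VR player proxy, built on the API example, that gives the player a hand-held menu and a weapon laser.
; On authority it puts a new or existing world menu on the off hand and a widget interactor on the dominant hand, then re-snaps the laser to the held item every second.
; CheckForMag respawns the held gun with or without a magazine, copying attachments.
; Death handling destroys pawn or interactor and menu; unconnected test and API nodes remain.
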(event `self.ReceiveTick`
  (params (DeltaSeconds :type "Float (single-precision)")))

(event `CheckAngle`
  (params (Rotation :type "Rotator Structure")))

(event `GiveLazer`
  (bind _lazer (`self.Lazer`))
  (bind _returnvalue (`|SpawnActorFromClass` "/Game/CustomMaps/UGC2842012712/Blueprints/lazer.lazer_C" (`KismetMathLibrary.MakeTransform` (0.0 0.0 0.0)) "Undefined" "OverrideRootScale" (`GameplayStatics.GetPlayerController` 0) null))
  (bind _output_get (set `self.Lazer` _returnvalue))
  (set `/Game/CustomMaps/UGC2842012712/Blueprints/lazer.Menu` (`self.MenuWidget`) _output_get)
  (set `/Game/CustomMaps/UGC2842012712/Blueprints/WidgetMenu/MainMenu.Lazer` _returnvalue (`self.MenuWidget`))
  (set `/Game/CustomMaps/UGC2842012712/Blueprints/lazer.PlayerProxy` self _returnvalue)
  (bind (_bhasitem _item) (`self.GetHeldItem` true :!label _label))
  (if _bhasitem
    (bind (_item_2 _itemname) (break `PlayerItem` _item))
    (if (`KismetStringLibrary.Contains` (`KismetStringLibrary.Conv_NameToString` _itemname) "AK47")
      (`self.K2_AttachToActor` _lazer _item_2 "Chamber" "SnapToTarget" "SnapToTarget" "KeepWorld" false)
      (else
        (`self.K2_AttachToActor` _lazer _item_2 "Muzzle" "SnapToTarget" "SnapToTarget" "KeepWorld" false))))
  (`KismetSystemLibrary.Delay` 1.0)
  (goto _label))

(event `AttachLazer`
  (goto _label))

(event `CheckForMag`
  (params (`IsChecked?` :type Boolean))
  (bind (_bhasitem _item) (`self.GetHeldItem` true))
  (for _array_element (`self.GetOverlappingActors` (break `PlayerItem` _item) null)
    (if (!= (`KismetStringLibrary.Contains` (`KismetSystemLibrary.GetClassDisplayName` (`GameplayStatics.GetObjectClass` _array_element)) "Magazine") `IsChecked?`)
      (`self.SpawnGun` `IsChecked?`))))

(event `SpawnGun`
  (params (`IsCkecked?` :type Boolean :default true))
  (bind _returnvalue (`Pavlov_Library.GetGameLogic`))
  (bind (_bhasitem _item) (`self.GetHeldItem` true))
  (if _bhasitem
    (bind _attachments (`self.GetWeaponAttachments` (break `PlayerItem` _item)))
    (bind _playerstatus (`PavlovProxyStatics.GetPavlovPlayerStatusByPawn` (`self.GetPawn`)))
    (bind (_bsuccessful _item_2) (`Pavlov_GameLogic.SpawnItemWRef` _returnvalue (make `PavlovItemSpawnParams` (`.ItemName` (break `PlayerItem` _item)) (break `PavlovPlayerStatus` _playerstatus) true false 0 false (struct) `IsCkecked?` false)))
    (`Pavlov_GameLogic.SpawnAttachments` _returnvalue (make `PavlovAttachmentSpawnParams` _attachments _item_2 false "None" (break `PavlovPlayerStatus` _playerstatus)))
    (`self.AttachLazer`)
    (`self.K2_DestroyActor` (break `PlayerItem` _item))))

(event `self.OnPlayerDeath`
  (params (KilledActor :type "Actor Object Reference"))
  ;[1 1 1] Called when the player dies, can clean up the body here by setting its life span
  (`/Engine/EditorBlueprintResources/ActorMacros.Switch Has Authority`
    (:`Authority`
      (`KismetSystemLibrary.PrintString` "player died server")
      (`self.K2_DestroyActor` (`self.GetPawn`)))
    (:`Remote`
      (`KismetSystemLibrary.PrintString` "player died client")
      (if (`KismetSystemLibrary.IsValid` (`self.Interactor`))
        (`self.K2_DestroyActor` (`self.Interactor`))
        (`self.K2_DestroyActor` (`self.Menu`))))))

(event `CallDoGiveInteractor`
  (`/Engine/EditorBlueprintResources/ActorMacros.Switch Has Authority`
    (:`Authority`
      (`KismetSystemLibrary.Delay` 2.0)
      (`self.DoGiveInteractor`)
      (`self.GiveLazer`))))

(event `DoGiveInteractor`
  (bind (_handsproxy_nondominanthand _handsproxy_dominanthand) (break `HandsProxy` (`self.HandsProxy`)))
  (bind _menus (`/Game/CustomMaps/UGC2842012712/GL_Deathmatch.Menus` (`self.GameLogic`)))
  (bind _output (`|GetArrayItem` _menus))
  (bind _returnvalue (`SceneComponent.GetAttachParent` (`SceneComponent.GetAttachParent` (`SceneComponent.GetAttachParent` _handsproxy_nondominanthand))))
  (bind _returnvalue_2 (`SceneComponent.GetAttachParent` (`SceneComponent.GetAttachParent` (`SceneComponent.GetAttachParent` _handsproxy_dominanthand))))
  (if (> (`KismetArrayLibrary.Array_Length` _menus) 0)
    (`self.K2_AttachToComponent` _output _returnvalue "None" "SnapToTarget" "SnapToTarget" "KeepRelative" false)
    (set `self.Menu` _output)
    (else
      (bind _returnvalue_3 (`|SpawnActorFromClass` "/Game/CustomMaps/UGC2842012712/Blueprints/WidgetMenu/VrWorldMenu.VrWorldMenu_C" (`SceneComponent.K2_GetComponentToWorld` _returnvalue) "Undefined" "OverrideRootScale" (`GameplayStatics.GetPlayerController` 0) self null))
      (bind _output_get (set `self.Menu` _returnvalue_3))
      (bind _asgl_deathmatch (cast `/Game/CustomMaps/UGC2842012712/GL_Deathmatch` (`Pavlov_Library.GetGameLogic`)))
      (`KismetArrayLibrary.Array_AddUnique` (`/Game/CustomMaps/UGC2842012712/GL_Deathmatch.Menus` _asgl_deathmatch) _returnvalue_3)
      (bind _asmain_menu (cast `/Game/CustomMaps/UGC2842012712/Blueprints/WidgetMenu/MainMenu` (`WidgetComponent.GetUserWidgetObject` (`/Game/CustomMaps/UGC2842012712/Blueprints/WidgetMenu/VrWorldMenu.Widget1` _returnvalue_3))))
      (set `/Game/CustomMaps/UGC2842012712/Blueprints/WidgetMenu/MainMenu.Player` self _asmain_menu)
      (set `self.MenuWidget` _asmain_menu)
      (`self.K2_AttachToComponent` _output_get _returnvalue "None" "SnapToTarget" "SnapToTarget" "KeepRelative" false)))
  (bind _returnvalue_4 (`|SpawnActorFromClass` "/Game/CustomMaps/UGC2842012712/Blueprints/WidgetMenu/WidgetInteractor.WidgetInteractor_C" (`SceneComponent.K2_GetComponentToWorld` _returnvalue_2) "Undefined" "OverrideRootScale" (`GameplayStatics.GetPlayerController` 0) null))
  (bind _output_get_2 (set `self.Interactor` _returnvalue_4))
  (set `/Game/CustomMaps/UGC2842012712/Blueprints/WidgetMenu/VrWorldMenu.WidgetInteractor` _output_get_2 (`self.Menu`))
  (`self.K2_AttachToComponent` _output_get_2 _returnvalue_2 "Suppressor" "SnapToTarget" "SnapToTarget" "KeepRelative" false))

(fn `GetMenu`
  (returns (MainMenu :type "/Game/CustomMaps/UGC2842012712/Blueprints/WidgetMenu/MainMenu Object Reference"))
  (return (`self.MenuWidget`)))

(fn `GetVoiceAttenuation`
  (returns (ReturnValue :type "SoundAttenuation Object Reference"))
  ;[1 1 1] Set attenuation here
  (return null))

(fn `UserConstructionScript`)