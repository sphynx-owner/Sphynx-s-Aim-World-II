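; Laser hit-scan actor for Pavlov target practice that registers shots on targets.
; Depending on the menu's count-bullets checkbox, a shot comes from a trigger pull with an item in that hand or a BulletCheck overlap, with mouse-button equivalents.
; LazerHit tries the beam mesh's overlapping TargetTemplate, then PracticeTemplate, then a debug-drawn multi line trace messaging the first BPI_HitScan actor.
; PlayerProxy handles held-item, magazine and angle checks.
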(event `Key|LeftMouseButton`
  (params (Key :type "Key Structure"))
  (:`Pressed`
    (if (== false (`CheckBox.IsChecked` (`/Game/CustomMaps/UGC2842012712/Blueprints/WidgetMenu/MainMenu.CheckBox_CountBullets?` (`self.Menu`)))) :!label _label
      (`self.LazerHit` false))))

(event `InputAction|TriggerRight` :consume false :overrideparent false
  (params (Key :type "Key Structure"))
  (:`Pressed`
    (`|ExecutionSequence`
      (:`then_0`
        (bind _playerstatus (`PavlovProxyStatics.GetPavlovPlayerStatusByPawn` (`Pavlov_PlayerProxy.GetPawn` (`self.PlayerProxy`)) :!label _label_2)))
      (:`then_1`
        (`self.CHeckHand` true)))))

(event `CHeckHand`
  (params (`RightHand?` :type Boolean))
  (bind _bhasitem (`Pavlov_PlayerProxy.GetHeldItem` (`self.PlayerProxy`) (not (xor `RightHand?` (`.bRightHanded` (break `PavlovPlayerStatus` (stale `InputAction|TriggerRight` _playerstatus)))))))
  (if _bhasitem
    (goto _label)))

(event `InputAction|TriggerLeft` :consume false :overrideparent false
  (params (Key :type "Key Structure"))
  (:`Pressed`
    (`|ExecutionSequence`
      (:`then_0`
        (goto _label_2))
      (:`then_1`
        (`self.CHeckHand` false)))))

(event `Key|RightMouseButton`
  (params (Key :type "Key Structure"))
  (bind (_returnvalue_roll _returnvalue_pitch _returnvalue_yaw) (`KismetMathLibrary.BreakRotator` (`SceneComponent.K2_GetComponentRotation` (`self.Scene`))))
  (:`Pressed`
    (if (== true (`CheckBox.IsChecked` (`/Game/CustomMaps/UGC2842012712/Blueprints/WidgetMenu/MainMenu.CheckBox_CountBullets?` (`self.Menu`)))) :!label _label_3
      (`self.LazerHit` true)
      (`/Game/CustomMaps/UGC2842012712/Blueprints/BP_PlayerProxyExample_1.CheckAngle` (`self.PlayerProxy`) (`KismetMathLibrary.MakeRotator` _returnvalue_roll _returnvalue_pitch _returnvalue_yaw)))))

(event `self.BulletCheck.OnComponentBeginOverlap`
  (params (OverlappedComponent :type "PrimitiveComponent Object Reference") (OtherActor :type "Actor Object Reference") (OtherComp :type "PrimitiveComponent Object Reference") (OtherBodyIndex :type Integer) (bFromSweep :type Boolean) (SweepResult :type "HitResult Structure (by ref)"))
  (goto _label_3))

(event `LazerHit`
  (params (`Bullet?` :type Boolean))
  (bind _astarget_template (cast `/Game/CustomMaps/UGC2842012712/Blueprints/Practices/TargetTemplate` (`|GetArrayItem` (`PrimitiveComponent.GetOverlappingActors` (`self.StaticMesh`) "/Game/CustomMaps/UGC2842012712/Blueprints/Practices/TargetTemplate.TargetTemplate_C")))
    (:`then`
      (bind _mainblueprint (`/Game/CustomMaps/UGC2842012712/Blueprints/Practices/TargetTemplate.MainBlueprint` _astarget_template))
      (if (and (`/Game/CustomMaps/UGC2842012712/Blueprints/Practices/PracticeTemplate.IsHitScan?` _mainblueprint) (`/Game/CustomMaps/UGC2842012712/Blueprints/Practices/PracticeTemplate.PracticeRunning?` _mainblueprint))
        (if (not `Bullet?`)
          (`/Game/CustomMaps/UGC2842012712/Blueprints/BP_PlayerProxyExample_1.CheckForMag` (`self.PlayerProxy`) `Bullet?`))
        (`/Game/CustomMaps/UGC2842012712/Blueprints/Practices/TargetTemplate.TargetHit` _astarget_template)
        (else
          (`self.CastToPractice` :!label _label_4))))
    (:`CastFailed`
      (goto _label_4))))

(event `CastToPractice`
  (bind _output (`|GetArrayItem` (`PrimitiveComponent.GetOverlappingActors` (`self.StaticMesh`) "/Game/CustomMaps/UGC2842012712/Blueprints/Practices/PracticeTemplate.PracticeTemplate_C")))
  (`KismetSystemLibrary.PrintString` (`KismetSystemLibrary.GetDisplayName` _output))
  (bind _aspractice_template (cast `/Game/CustomMaps/UGC2842012712/Blueprints/Practices/PracticeTemplate` _output)
    (:`then`
      (if (`/Game/CustomMaps/UGC2842012712/Blueprints/Practices/PracticeTemplate.IsHitScan?` _aspractice_template)
        (if (not (stale `LazerHit` `Bullet?`))
          (`/Game/CustomMaps/UGC2842012712/Blueprints/BP_PlayerProxyExample_1.CheckForMag` (`self.PlayerProxy`) (stale `LazerHit` `Bullet?`)))
        (`/Game/CustomMaps/UGC2842012712/Blueprints/Practices/PracticeTemplate.HitScan` _aspractice_template self)))
    (:`CastFailed`
      (bind _outhits (`KismetSystemLibrary.LineTraceMultiForObjects` :`Start` (`SceneComponent.K2_GetComponentLocation` (`self.Origin`)) :`End` (`SceneComponent.K2_GetComponentLocation` (`self.End`)) :`ObjectTypes` (`|MakeArray` "ObjectTypeQuery2" "ObjectTypeQuery1" :!type "EObjectTypeQuery Enum") :`bTraceComplex` true :`DrawDebugType` "ForDuration"))
      (for _array_element _outhits
        (bind (_bblockinghit _binitialoverlap _time _distance _location _impactpoint _normal _impactnormal _physmat _hitactor) (`GameplayStatics.BreakHitResult` _array_element))
        (if (`KismetSystemLibrary.DoesImplementInterface` _hitactor "/Game/CustomMaps/UGC2842012712/Blueprints/Global/Interfaces/BPI_HitScan.BPI_HitScan_C")
          (`|ExecutionSequence`
            (:`then_0`
              (break))
            (:`then_1`
              (message `/Game/CustomMaps/UGC2842012712/Blueprints/Global/Interfaces/BPI_HitScan.BPIHitScan` _hitactor _array_element (stale `LazerHit` `Bullet?`)))))))))

(fn `UserConstructionScript`)