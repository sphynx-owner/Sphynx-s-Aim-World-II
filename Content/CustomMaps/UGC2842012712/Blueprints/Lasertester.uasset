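; Lasertester is a test actor that fills a vertical plane with 400 Lazer actors when play begins.
; A BeginPlay loop spawns each Lazer rotated, attaches it to the tester and makes its static mesh visible.
; Modulo and truncated division on the centered loop index set relative X and Z in fixed steps, forming a grid whose two halves overlap at the middle row.
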(event `self.ReceiveBeginPlay`
  (for _index (range 400)
    (bind _returnvalue (`|SpawnActorFromClass` "/Game/CustomMaps/UGC2842012712/Blueprints/lazer.lazer_C" (`KismetMathLibrary.MakeTransform` (0.0 0.0 0.0) (struct :`Yaw` 90.0)) "Undefined" "OverrideRootScale" null null))
    (`self.K2_AttachToActor` _returnvalue self "None" "SnapToTarget" "KeepRelative" "KeepRelative" false)
    (bind _returnvalue_2 (- (`KismetMathLibrary.Conv_IntToDouble` _index) 200.0))
    (`SceneComponent.K2_SetRelativeLocation` (`Actor.RootComponent` _returnvalue) (`KismetMathLibrary.MakeVector` (* (- (`KismetMathLibrary.Abs` (mod _returnvalue_2 20.0)) 20.0) 50.0) 0.0 (* (`KismetMathLibrary.Conv_IntToDouble` (`KismetMathLibrary.FTrunc` (/ _returnvalue_2 20.0))) 50.0)) false false)
    (`SceneComponent.SetVisibility` (`/Game/CustomMaps/UGC2842012712/Blueprints/lazer.StaticMesh` _returnvalue) true false)))

(fn `UserConstructionScript`
  (locals (NewLocalVar_0 :type "Viewport Object Reference")))